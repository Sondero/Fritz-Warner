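; Interactive swinging door Blueprint that toggles open and closed on interaction and closes itself after a delay.
; The first interaction caches the current yaw as the closed angle.
; The Opener timeline plays or reverses to drive the actor's yaw by OpenAngle from that baseline.
; Tick starts a CloseTime Delay while open, then calls AutomaticClose, with no cancellation on manual closing.
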(event `Interraction`
  (bind _returnvalue (not (`self.Open?`)))
  (if (`self.Has opened once`)
    (bind _output_get (set `self.Open?` _returnvalue))
    (if _output_get
      (bind (_direction _door_progress) (`Timeline|Opener` :!label _label)
        (:`Update`
          (`self.K2_SetActorRotation` (`KismetMathLibrary.MakeRotator` 0.0 0.0 (+ (* _door_progress (`self.OpenAngle`)) (`self.ClosedAngle`))))
          (set `self.Has opened once` true)))
      (else
        (goto _label :!via `Reverse`)))
    (else
      (set `self.Open?` _returnvalue)
      (set `self.ClosedAngle` (.yaw (`self.K2_GetActorRotation`)))
      (goto _label))))

(event `Automatic Close`
  (set `self.Open?` false)
  (goto _label :!via `Reverse`))

(event `self.ReceiveTick`
  (params (DeltaSeconds :type "Float (single-precision)"))
  (if (`self.Open?`)
    (`KismetSystemLibrary.Delay` (`self.Close time`))
    (`self.Automatic Close`)))

(fn `UserConstructionScript`)