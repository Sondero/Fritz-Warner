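; A power switch that toggles a linked object, such as a door, open or closed when an Electric_Bullet overlaps it.
; A timeline slides the InterractionObject between its start location and a relative target, playing forward or in reverse.
; A box component added to that object at BeginPlay halts closing while the player is inside it and kills any Enemy caught there.
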(event `self.ReceiveBeginPlay`
  (bind _interraction_object (`self.Interraction Object`))
  (bind _output_get (set `self.StartLocation` (`self.K2_GetActorLocation` _interraction_object)))
  (set `self.TargetLocation` (+ _output_get (`self.Relative Target Location`)))
  (bind _returnvalue (`AddComponent|NODE_AddBoxComponent-0` :`self` _interraction_object :`RelativeTransform` (`KismetMathLibrary.MakeTransform` (0.0 0.0 -20.0) (struct) (1.45 1.45 1.8))))
  (set `self.ClosingSafety` _returnvalue))

(event `self.ReceiveActorBeginOverlap`
  (params (OtherActor :type "Actor Object Reference"))
  (cast `/Game/ThirdPersonCPP/Blueprints/Electric_Bullet` OtherActor)
  (bind _output_get (set `self.Open?` (not (`self.Open?`))))
  (if _output_get
    (bind (_direction _moving) (`Timeline|Moving%` :!label _label)
      (:`Update`
        ;[1 1 1] Stops the Door from closing if the Player is about to get trapped
        (if (and (`PrimitiveComponent.IsOverlappingActor` (`self.ClosingSafety`) (`GameplayStatics.GetPlayerPawn` 0)) (== (`self.Open?`) false))
          (goto _label :!via `Stop`)
          (else
            (set `self.MomentaryTargetLocation` (+ (`self.StartLocation`) (* (- (`self.TargetLocation`) (`self.StartLocation`)) _moving)))
            (`self.K2_SetActorLocation` (`self.Interraction Object`) (`self.MomentaryTargetLocation`) false false)
            (if (== (`self.Open?`) false)
              ;[1 1 1] Kills Enemies that are getting trapped by the door
              (for _array_element (`PrimitiveComponent.GetOverlappingActors` (`self.ClosingSafety`) "/Game/Blueprints/Enemy/Enemy.Enemy_C")
                (bind _asenemy (cast `/Game/Blueprints/Enemy/Enemy` _array_element))
                (`/Game/Blueprints/Enemy/Enemy.OnDeath` _asenemy)))))))
    (else
      (goto _label :!via `Reverse`))))

(fn `UserConstructionScript`)