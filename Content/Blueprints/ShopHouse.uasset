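; ShopHouse is an enterable shop building with a swinging door that opens a shop menu when the player walks inside.
; ActivateDoor toggles a timeline that rotates the door from a closed yaw captured on first use, and Tick auto-closes it after a delay.
; Overlapping the InsideShop trigger pauses the game and shows the Shop widget with UI-only input, passing it an exit location computed at BeginPlay.
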(event `self.ReceiveBeginPlay`
  (set `self.Location for Exit (Actor)` (+ (`self.K2_GetActorLocation`) (`self.DoorLocation`))))

(event `self.InsideShop.OnComponentBeginOverlap`
  (params (OverlappedComponent :type "PrimitiveComponent Object Reference") (OtherActor :type "Actor Object Reference") (OtherComp :type "PrimitiveComponent Object Reference") (OtherBodyIndex :type Integer) (bFromSweep :type Boolean) (SweepResult :type "HitResult Structure (by ref)"))
  (bind _returnvalue (`GameplayStatics.GetPlayerController` 0))
  (cast `/Game/ThirdPersonCPP/Blueprints/ThirdPersonCharacter` OtherActor)
  (`GameplayStatics.SetGamePaused` true)
  (bind _returnvalue_2 (`|CreateWidget` "/Game/Blueprints/UI/Shop.Shop_C" _returnvalue))
  (set `/Game/Blueprints/UI/Shop.ExitLocation` (`self.Location for Exit (Actor)`) _returnvalue_2)
  (`UserWidget.AddToViewport` _returnvalue_2 0)
  (`WidgetBlueprintLibrary.SetInputMode_UIOnlyEx` _returnvalue _returnvalue_2)
  (set `PlayerController.bShowMouseCursor` true _returnvalue))

(event `ActivateDoor`
  (bind _returnvalue (not (`self.Open?`)))
  ;[1 1 1] Door
  (if (`self.Has opened once`)
    (bind _output_get (set `self.Open?` _returnvalue))
    (if _output_get
      (bind (_direction _door_progress) (`Timeline|Opener` :!label _label)
        (:`Update`
          (`SceneComponent.K2_SetWorldRotation` (`self.ShopDoor`) (`KismetMathLibrary.MakeRotator` 0.0 0.0 (+ (* _door_progress (`self.OpenAngle`)) (`self.ClosedAngle`))) false false)
          (set `self.Has opened once` true)))
      (else
        (goto _label :!via `Reverse`)))
    (else
      (set `self.Open?` _returnvalue)
      (set `self.ClosedAngle` (.yaw (`SceneComponent.K2_GetComponentRotation` (`self.ShopDoor`))))
      (goto _label))))

(event `Automatic Close`
  ;[1 1 1] Door
  (set `self.Open?` false)
  (goto _label :!via `Reverse`))

(event `self.ReceiveTick`
  (params (DeltaSeconds :type "Float (single-precision)"))
  ;[1 1 1] Door
  (if (`self.Open?`)
    (`KismetSystemLibrary.Delay` (`self.Close time`))
    (`self.Automatic Close`)))

(fn `UserConstructionScript`)